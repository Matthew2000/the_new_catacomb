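; BP_SplineBuilder is a construction-time tool that lays repeated copies of a mesh along the segments of a spline.
; The construction script makes spline points linear and adds an instanced static mesh component at each point, offset by MeshOffset.
; Each segment's X delta, or Y as fallback, divided by MeshWidth sets how many rotated instances step along that component's local X.
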(event EventBeginPlay)

(event Collision|EventActorBeginOverlap
  (params (OtherActor :type Actor%20Object%20Reference)))

(event EventTick
  (params (DeltaSeconds :type Float%20%28single-precision%29)))

(fn ConstructionScript
  (bind _spline (Variables|Default|GetSpline))
  (bind _spline_2 (Variables|Default|GetSpline))
  (bind _meshwidth (Variables|Default|GetMeshWidth))
  (bind _returnvalue (Spline|GetNumberOfSplinePoints _spline))
  (if (>= _returnvalue 2)
    (for _index (range 0 _returnvalue)
      (Spline|SetSplinePointType _spline_2 _index "Linear" true)
      (bind _returnvalue_2 (AddComponent|AddInstancedStaticMeshComponent false (Math|Transform|ComposeTransforms (Variables|Default|GetMeshOffset) (Spline|GetTransformatSplinePoint _spline_2 _index "Local" false))))
      (Components|StaticMesh|SetStaticMesh _returnvalue_2 (Variables|Default|GetMesh))
      (if (and (!= (.x (- (.Location (Math|Transform|BreakTransform (Spline|GetTransformatSplinePoint _spline_2 (+ _index 1) "Local" false))) (.Location (Math|Transform|BreakTransform (Spline|GetTransformatSplinePoint _spline_2 _index "Local" false))))) 0.0) (> (Math|Integer|Absolute(Integer) (Math|Float|Truncate (/ (.x (- (.Location (Math|Transform|BreakTransform (Spline|GetTransformatSplinePoint _spline_2 (+ _index 1) "Local" false))) (.Location (Math|Transform|BreakTransform (Spline|GetTransformatSplinePoint _spline_2 _index "Local" false))))) _meshwidth))) 0))
        (for _index_2 (range 1 (Math|Integer|Absolute(Integer) (Math|Float|Truncate (/ (.x (- (.Location (Math|Transform|BreakTransform (Spline|GetTransformatSplinePoint _spline_2 (+ _index 1) "Local" false))) (.Location (Math|Transform|BreakTransform (Spline|GetTransformatSplinePoint _spline_2 _index "Local" false))))) _meshwidth))))
          (Components|InstancedStaticMesh|AddInstance _returnvalue_2 (Math|Transform|MakeTransform (Math|Vector|MakeVector (* _index_2 _meshwidth) 0.0 0.0) "0,90.000000, 0" "1,1,1")))
        (elif (and (!= (.y (- (.Location (Math|Transform|BreakTransform (Spline|GetTransformatSplinePoint _spline_2 (+ _index 1) "Local" false))) (.Location (Math|Transform|BreakTransform (Spline|GetTransformatSplinePoint _spline_2 _index "Local" false))))) 0.0) (> (Math|Integer|Absolute(Integer) (Math|Float|Truncate (/ (.y (- (.Location (Math|Transform|BreakTransform (Spline|GetTransformatSplinePoint _spline_2 (+ _index 1) "Local" false))) (.Location (Math|Transform|BreakTransform (Spline|GetTransformatSplinePoint _spline_2 _index "Local" false))))) _meshwidth))) 0))
          (for _index_3 (range 1 (Math|Integer|Absolute(Integer) (Math|Float|Truncate (/ (.y (- (.Location (Math|Transform|BreakTransform (Spline|GetTransformatSplinePoint _spline_2 (+ _index 1) "Local" false))) (.Location (Math|Transform|BreakTransform (Spline|GetTransformatSplinePoint _spline_2 _index "Local" false))))) _meshwidth))))
            (Components|InstancedStaticMesh|AddInstance _returnvalue_2 (Math|Transform|MakeTransform (Math|Vector|MakeVector (* _index_3 _meshwidth) 0.0 0.0) "0,90.000000, 0" "1,1,1"))))))))