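; BP_Save is a save object that snapshots and restores the player's location, spotlight visibility, oil, sanity and stamina.
; The save event copies that state, appends the passed interactables to its array, then writes itself to the named slot.
; The load event applies the stored values to the player and disconnects their rope, but does not read the slot or use the interactables array.
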(event Custom|save
  (params (player :type First%20Person%20Character%20Object%20Reference) (inters :type Array%20of%20Interactable%20Save%20Structures) (save_name :type String))
  (bind _self self)
  ;[1 1 1] save
  (Variables|BP_Save_C|SetLocation_save _self (Transformation|GetActorLocation player))
  (Variables|BP_Save_C|Setlamp_save _self (Rendering|IsVisible (Variables|/Game/FirstPersonCPP/Blueprints/FirstPersonCharacter.FirstPersonCharacter_C|GetSpotLight player)))
  (Variables|BP_Save_C|Setoil_save _self (Variables|/Script/the_new_catacomb.the_new_catacombCharacter|GetOilLevel player))
  (Variables|BP_Save_C|Setsanity_save _self (Variables|/Script/the_new_catacomb.the_new_catacombCharacter|GetSanity player))
  (Variables|BP_Save_C|Setstamina_save _self (Variables|/Script/the_new_catacomb.the_new_catacombCharacter|GetStamina player))
  (for _array_element inters
    (Utilities|Array|Add (Variables|Default|GetInteractables) _array_element))
  (SaveGame|SaveGametoSlot _self save_name))

(event Custom|load
  (params (player :type First%20Person%20Character%20Object%20Reference))
  (bind _self self)
  ;[1 1 1] load
  (Transformation|SetActorLocation player (Variables|BP_Save_C|GetLocation_save _self) false false)
  (Rendering|SetVisibility (Variables|/Game/FirstPersonCPP/Blueprints/FirstPersonCharacter.FirstPersonCharacter_C|GetSpotLight player) (Variables|BP_Save_C|Getlamp_save _self) false)
  (Variables|/Script/the_new_catacomb.the_new_catacombCharacter|SetOilLevel player (Variables|BP_Save_C|Getoil_save _self))
  (Variables|/Script/the_new_catacomb.the_new_catacombCharacter|SetSanity player (Variables|BP_Save_C|Getsanity_save _self))
  (Variables|/Script/the_new_catacomb.the_new_catacombCharacter|SetStamina player (Variables|BP_Save_C|Getstamina_save _self))
  (Default|DisconnectRope player))