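; BP_BaseItem is the base pickup item, a BP_BaseInteractable child that players can target and collect.
; On interaction it passes its ItemInfo struct to the instigator via PickupItemMessage, prints a pickup message and destroys itself.
; It overrides SetFeedback to print the item's name when targeted or untargeted.
; The construction script writes the actor's own class into ItemInfo, so each child item records its class automatically.
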(event EventSetFeedback
  (params (GiveFeedback :type Boolean))
  (bind _iteminfo (Variables|Default|GetItemInfo))
  (if GiveFeedback
    (Development|PrintText (.itemname _iteminfo) true true "(R=0.022775,G=1.000000,B=0.000000,A=1.000000)" 3.0)
    (else
      (Development|PrintText (Utilities|Text|FormatText "{ItemName} was untargetted." (.itemname _iteminfo)) true true "(R=1.000000,G=0.000000,B=0.038008,A=1.000000)"))))

(event EventInteraction
  (params (Instigator :type First%20Person%20Character%20Object%20Reference))
  (Class|BPIInteractor|PickupItem(Message) Instigator (Variables|Default|GetItemInfo))
  (Development|PrintText (Utilities|Text|FormatText "{ItemName} was picked up." (.itemname (Variables|Default|GetItemInfo))) true true "(R=1.000000,G=0.779124,B=0.000000,A=1.000000)" 3.0)
  (Actor|DestroyActor))

(fn ConstructionScript
  ;[1 1 1] This logic is automatically getting reference to 'self' in the children of this class
  (|CallParentFunction)
  (Variables|Default|SetItemInfo (Utilities|Struct|MakeFItemInfo (.itemname (Variables|Default|GetItemInfo)) (.itemtype (Variables|Default|GetItemInfo)) (.itemimg (Variables|Default|GetItemInfo)) (Utilities|GetClass self) (.itemdescrip (Variables|Default|GetItemInfo)))))