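; Base Blueprint for interactable objects that the first-person player can target.
; When the player overlaps or leaves its collider, it registers or unregisters itself with the FirstPersonCharacter through BPI_Interactor interface messages.
; SetFeedback prints placeholder targeted and untargeted messages, and child items override it to display their names.
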(event OnComponentBeginOverlap(InteractableCollider)
  (params (OverlappedComponent :type Primitive%20Component%20Object%20Reference) (OtherActor :type Actor%20Object%20Reference) (OtherComp :type Primitive%20Component%20Object%20Reference) (OtherBodyIndex :type Integer) (bFromSweep :type Boolean) (SweepResult :type Hit%20Result%20Structure%20%28by%20ref%29))
  ;[1 1 1] When the player's collider interacts with the interactable's collider, send this
  ; Object's reference to the player
  (bind _asfirst_person_character (Utilities|Casting|CastToFirstPersonCharacter OtherActor))
  (Class|BPIInteractor|RegisterInteractables(Message) _asfirst_person_character self) ; This function was created in an interface (BPI_Interactor) and is \nbeing used to send references across blueprints.
)

(event OnComponentEndOverlap(InteractableCollider)
  (params (OverlappedComponent :type Primitive%20Component%20Object%20Reference) (OtherActor :type Actor%20Object%20Reference) (OtherComp :type Primitive%20Component%20Object%20Reference) (OtherBodyIndex :type Integer))
  ;[1 1 1] When the player's collider interacts with the interactable's collider, send this
  ; Object's reference to the player
  (bind _asfirst_person_character (Utilities|Casting|CastToFirstPersonCharacter OtherActor))
  (Class|BPIInteractor|UnregisterInteractables(Message) _asfirst_person_character self))

(fn ConstructionScript)

(fn SetFeedback
  (params (GiveFeedback :type Boolean))
  (if GiveFeedback
    (Development|PrintString "Interactable Targetted" true true "(R=0.000000,G=0.660000,B=1.000000,A=1.000000)" 3.0)
    (else
      (Development|PrintString "Interactable no longer targeted" true true "(R=1.000000,G=0.047707,B=0.000000,A=1.000000)" 3.0))))