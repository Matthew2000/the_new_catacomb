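; Interactable rest area that lets the interacting character rest behind a screen fade.
; On interaction it disables the instigator's movement, fades the camera out, calls Rest on the instigator, then fades back in and re-enables movement.
; A DoOnce gate blocks repeat interactions until the fade-in finishes.
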(event EventInteraction
  (params (Instigator :type First%20Person%20Character%20Object%20Reference))
  (bind _fadeouttime (Variables|Default|GetFadeOutTime))
  (bind _charactermovement (Variables|/Script/Engine.Character|GetCharacterMovement Instigator))
  (Utilities|FlowControl|DoOnce false :!label _label
    (:Completed
      (Components|Activation|SetActive _charactermovement false false)
      (Utilities|FlowControl|Sequence
        (:then_0
          (CameraFades|StartCameraFade :self (Game|GetPlayerCameraManager 0) :ToAlpha 1.0 :Duration _fadeouttime :bHoldWhenFinished true))
        (:then_1
          (Utilities|FlowControl|Delay _fadeouttime)
          (Class|TheNewCatacombCharacter|Rest Instigator)
          (Utilities|FlowControl|Delay 0.5)
          (CameraFades|StartCameraFade :self (Game|GetPlayerCameraManager 0) :FromAlpha 1.0 :Duration (Variables|Default|GetFadeInTime))
          (Components|Activation|SetActive _charactermovement true false)
          (Utilities|FlowControl|Delay (Variables|Default|GetFadeInTime))
          (goto _label Reset))))))

(fn ConstructionScript
  (|CallParentFunction))

(fn NewFunction0)