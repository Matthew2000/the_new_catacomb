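; Interactable torch that an instigator with a lamp can light and that restores the first-person player's sanity while lit.
; Interaction reveals the fire effect and point light if the torch is unlit, with no path to extinguish it.
; Tick uses a Delay to check about once per second whether the player is horizontally near the visible light, then slightly raises Sanity.
; The SetFeedback event is left empty.
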(event EventTick
  (params (DeltaSeconds :type Float%20%28single-precision%29))
  (Utilities|FlowControl|Delay 1.0)
  (bind _asfirst_person_character (Utilities|Casting|CastToFirstPersonCharacter (Game|GetPlayerCharacter 0)))
  (if (and (< (Math|Vector|Distance2D(Vector) (Transformation|GetActorLocation _asfirst_person_character) (Transformation|GetWorldLocation (Variables|Default|GetTorch_PointLight))) 5e+02) (Rendering|IsVisible (Variables|Default|GetTorch_PointLight)))
    (Variables|/Script/the_new_catacomb.the_new_catacombCharacter|SetSanity _asfirst_person_character (+ (Variables|/Script/the_new_catacomb.the_new_catacombCharacter|GetSanity _asfirst_person_character) 0.01))))

(event EventSetFeedback
  (params (GiveFeedback :type Boolean)))

(event EventInteraction
  (params (Instigator :type First%20Person%20Character%20Object%20Reference))
  (if (and (Variables|/Game/FirstPersonCPP/Blueprints/FirstPersonCharacter.FirstPersonCharacter_C|GetLamp Instigator) (not (Variables|/Script/Engine.SceneComponent|GetbVisible (Variables|Default|GetTorch_PointLight))))
    (Rendering|SetVisibility (Variables|Default|GetP_Torch_Fire) true false)
    (Rendering|SetVisibility (Variables|Default|GetTorch_PointLight) true false)))

(fn ConstructionScript
  (|CallParentFunction))