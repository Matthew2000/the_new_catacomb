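; Interactable fire altar that a player carrying matches can light, showing its torch fire and point light.
; Interaction stores the player reference, and the match decrement is disconnected, so lighting costs nothing.
; Tick sets that player's InLight while inside the sphere, without checking whether the altar is lit; leaving clears it.
; The construction script sizes the sphere and light attenuation from separate radius variables.
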(event OnComponentEndOverlap(Sphere)
  (params (OverlappedComponent :type Primitive%20Component%20Object%20Reference) (OtherActor :type Actor%20Object%20Reference) (OtherComp :type Primitive%20Component%20Object%20Reference) (OtherBodyIndex :type Integer))
  (bind _asfirst_person_character (Utilities|Casting|CastToFirstPersonCharacter OtherActor))
  (Variables|/Script/the_new_catacomb.the_new_catacombCharacter|SetInLight _asfirst_person_character false))

(event EventTick
  (params (DeltaSeconds :type Float%20%28single-precision%29))
  (if (Collision|IsOverlappingActor (Variables|Default|GetSphere) (Variables|Default|GetPlayerRef) :!class /Script/Engine.PrimitiveComponent)
    (Variables|/Script/the_new_catacomb.the_new_catacombCharacter|SetInLight (Variables|Default|GetPlayerRef) true)))

(event EventInteraction
  (params (Instigator :type First%20Person%20Character%20Object%20Reference))
  (bind _output_get (Variables|Default|SetPlayerRef Instigator))
  (if (and (> (Variables|/Script/the_new_catacomb.the_new_catacombCharacter|GetMatches _output_get) 0) (not (Rendering|IsVisible (Variables|Default|GetTorch_PointLight))))
    (Rendering|SetVisibility (Variables|Default|GetP_Torch_Fire) true false)
    (Rendering|SetVisibility (Variables|Default|GetTorch_PointLight) true false)))

(fn ConstructionScript
  (|CallParentFunction)
  (Components|Sphere|SetSphereRadius (Variables|Default|GetSphere) (Variables|Default|GetLightRadius) true)
  (Rendering|Lighting|SetAttenuationRadius (Variables|Default|GetTorch_PointLight) (Variables|Default|GetPointLineRadius)))