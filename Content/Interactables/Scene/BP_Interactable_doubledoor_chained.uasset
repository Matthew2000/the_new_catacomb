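; BP_Interactable_doubledoor_chained is an interactable double door that opens once when Interaction fires while an overlap is active on its Box.
; Box overlaps set the In flag, and the Open timeline sets IfOpen when finished, with no closing path.
; Each timeline update adds the track value to DoorRight's current yaw cumulatively, and DoorLeft's rotation derives from DoorRight's rather than its own.
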(event OnComponentBeginOverlap(Box)
  (params (OverlappedComponent :type Primitive%20Component%20Object%20Reference) (OtherActor :type Actor%20Object%20Reference) (OtherComp :type Primitive%20Component%20Object%20Reference) (OtherBodyIndex :type Integer) (bFromSweep :type Boolean) (SweepResult :type Hit%20Result%20Structure%20%28by%20ref%29))
  (Variables|Default|Setin true)
  (Development|PrintString "is in door open range"))

(event OnComponentEndOverlap(Box)
  (params (OverlappedComponent :type Primitive%20Component%20Object%20Reference) (OtherActor :type Actor%20Object%20Reference) (OtherComp :type Primitive%20Component%20Object%20Reference) (OtherBodyIndex :type Integer))
  (Variables|Default|Setin false)
  (Development|PrintString "is out of door open range"))

(event EventInteraction
  (params (Instigator :type First%20Person%20Character%20Object%20Reference))
  (bind _doorright (Variables|Default|GetDoorRight))
  (bind _returnvalue (Transformation|GetRelativeTransform _doorright))
  (bind _rotation (Math|Transform|BreakTransform _returnvalue))
  (bind (_roll _pitch _yaw) (Math|Rotator|BreakRotator _rotation))
  (if (Variables|Default|Getin)
    (if (not (Variables|Default|Getif_open))
      (Development|PrintString "opening door")
      (bind _open (Timeline|open Play)
        (:Update
          (Transformation|SetRelativeRotation _doorright (Math|Rotator|MakeRotator _roll _pitch (+ _yaw _open)) false false)
          (Transformation|SetRelativeRotation (Variables|Default|GetDoorLeft) (Math|Rotator|MakeRotator _roll _pitch (+ _yaw _open)) false false))
        (:Finished
          (Variables|Default|Setif_open true))))))

(fn ConstructionScript
  (|CallParentFunction))